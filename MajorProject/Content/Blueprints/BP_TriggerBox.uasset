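; Trigger box Blueprint with a time check that picks a difficulty from the elapsed time reported by MajorProjectGameMode.
; FCheckTime prints the time and compares whole seconds to a short threshold, setting the Easy flag at or above it and Hard below; Medium is always cleared.
; The overlap event is empty, nothing here calls FCheckTime, and a print-only copy of the check sits unconnected in the event graph.
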(event `self.ReceiveActorBeginOverlap`
  (params (OtherActor :type "Actor Object Reference")))

(fn `f_CheckTime`
  (bind _asmajor_project_game_mode (cast `MajorProjectGameMode` (`GameplayStatics.GetGameMode`)))
  (bind _returnvalue (`MajorProjectGameMode.GetElapedTime` _asmajor_project_game_mode true false))
  (bind _returnvalue_2 (`MajorProjectGameMode.GetSecondsInt` _asmajor_project_game_mode))
  (if (>= _returnvalue_2 3)
    (`KismetSystemLibrary.PrintString` (`KismetStringLibrary.Conv_IntToString` _returnvalue) true true (struct :`R` 1.0 :`A` 1.0))
    (set `self.m_EasyDifficulty` true)
    (set `self.m_MediumDifficulty` false)
    (set `self.m_HardDifficulty` false)
    (else
      (`KismetSystemLibrary.PrintString` (`KismetStringLibrary.Conv_IntToString` _returnvalue) true true (struct :`G` 1.0 :`A` 1.0))
      (set `self.m_EasyDifficulty` false)
      (set `self.m_MediumDifficulty` false)
      (set `self.m_HardDifficulty` true))))

(fn `UserConstructionScript`)